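; BP_Turret is an automated turret that aims and fires bullets at the first-person player character when it sees them.
; PawnSensing sightings snap the actor's rotation toward a predicted position, using the player's velocity and bullet travel time, lowered by a fixed offset.
; After a short delay, it spawns BP_Bullet at the Arrow only if the player is falling, scaling projectile velocity by BulletsSpeed.
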(event `self.PawnSensing.OnSeePawn`
  (params (Pawn :type "Pawn Object Reference"))
  (bind _asbp_first_person_character (cast `/Game/FirstPerson/Blueprints/BP_FirstPersonCharacter` Pawn))
  (`self.K2_SetActorRotation` (`KismetMathLibrary.FindLookAtRotation` (`SceneComponent.K2_GetComponentLocation` (`self.Arrow`)) (+ (- (`SceneComponent.K2_GetComponentLocation` (`Character.CapsuleComponent` _asbp_first_person_character)) (0.0 0.0 96.0)) (* (`self.GetVelocity` _asbp_first_person_character) (/ (`self.GetDistanceTo` _asbp_first_person_character) (`self.bulletsSpeed`))))))
  (`KismetSystemLibrary.Delay` 0.5)
  (if (`NavMovementComponent.IsFalling` (`Character.CharacterMovement` _asbp_first_person_character))
    (bind _returnvalue (`|SpawnActorFromClass` "/Game/machine_gun/BP_Bullet.BP_Bullet_C" (`SceneComponent.K2_GetComponentToWorld` (`self.Arrow`)) "Undefined" "MultiplyWithRoot" null null))
    (bind _projectilemovement (`/Game/machine_gun/BP_Bullet.ProjectileMovement` _returnvalue))
    (set `MovementComponent.Velocity` (* (`MovementComponent.Velocity` _projectilemovement) (`self.bulletsSpeed`)) _projectilemovement)))

(fn `UserConstructionScript`)